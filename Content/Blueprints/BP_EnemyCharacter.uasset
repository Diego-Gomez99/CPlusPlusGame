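; Skeleton enemy character that attacks the player with a sword, takes damage and drops pickups on death.
; Sword hits use a sphere trace, and the player's EnemyFlinch flag triggers knockback on the enemy.
; Damage briefly shows the health bar; death leaves the player's enemy array, may drop health or arrows, then explodes.
; Player reference and health-bar setup are unwired from BeginPlay, so they never run.
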(event Custom|Attack
  ;[0.1562 1 0.5953] Enemy make damage
  (if (not (<= (Variables|Default|GetSkullHealth) 0.0))
    (Animation|PlayAnimMontage "/Game/CityofBrass_Enemies/Meshes/Enemy/Corpse/animation/BaseAttack.BaseAttack" 1.0 "None")))

(event Custom|CorpseSwordDamage
  (bind _corpsesword (Variables|Default|GetCorpseSword))
  (bind _playerref (Variables|Default|GetPlayerRef))
  (bind _returnvalue (Transformation|GetSocketLocation _corpsesword "None"))
  ;[0.1562 1 0.5953] Enemy make damage
  (bind _outactors (Actor|GetAllActorswithTag "Corpse"))
  (bind (_outhit _returnvalue_2) (Collision|SphereTraceByChannel _returnvalue _returnvalue 5e+01 "TraceTypeQuery1" false _outactors "ForDuration" true "(R=0.822917,G=0.152981,B=0.062706,A=1.000000)" "(R=1.000000,G=0.925346,B=0.000000,A=1.000000)"))
  (if _returnvalue_2
    (Variables|Default|SetPlayerImpactPoint (.ImpactPoint (Collision|BreakHitResult _outhit))) ; Save impact point from enemy to player
    (Game|Damage|ApplyDamage (.HitActor (Collision|BreakHitResult _outhit)) 2e+01 (Game|GetInstigatorController (.HitActor (Collision|BreakHitResult _outhit))) self)
    (if (Variables|/Game/ThirdPersonBP/Blueprints/Mycharacter.Mycharacter_C|GetEnemyFlinch _playerref)
      (CallFunction|Retroceder)
      (Variables|/Game/ThirdPersonBP/Blueprints/Mycharacter.Mycharacter_C|SetEnemyFlinch _playerref false))))

(event Custom|Retroceder
  (bind _playerref (Variables|Default|GetPlayerRef))
  (bind _returnvalue (Transformation|GetActorForwardVector _playerref))
  (bind _returnvalue_2 (* _returnvalue 1.5e+03))
  (Variables|Default|SetIsFlinching true)
  (Animation|PlayAnimMontage "/Game/CityofBrass_Enemies/Meshes/Enemy/Corpse/animation/Corpse_ClincMontage.Corpse_ClincMontage" 1.0 "None")
  (Character|LaunchCharacter (Math|Vector|MakeVector (.x _returnvalue_2) (.y _returnvalue_2) 0.0) false false)
  (Utilities|FlowControl|Delay 2.0)
  (Variables|Default|SetIsFlinching false))

(event EventBeginPlay
  ;[0.1816 1 0.351] Begin Play
)

(event Game|Damage|EventAnyDamage
  (params (Damage :type Float%20%28single-precision%29) (DamageType :type Damage%20Type%20Object%20Reference) (InstigatedBy :type Controller%20Object%20Reference) (DamageCauser :type Actor%20Object%20Reference))
  (bind _health (Variables|Default|GetHealth))
  (bind _playerref (Variables|Default|GetPlayerRef))
  (bind _enemiesref (Variables|/Game/ThirdPersonBP/Blueprints/Mycharacter.Mycharacter_C|GetEnemiesRef _playerref))
  ;[1 0.1292 0.2289] Enemy Get Damaged
  (bind _output_get (Variables|Default|SetSkullHealth (- (Variables|Default|GetSkullHealth) Damage)))
  (if (<= _output_get 0.0)
    (Utilities|FlowControl|DoOnce false
      (:Completed
        (Pawn|Components|CharacterMovement|DisableMovement (Variables|Character|GetCharacterMovement))
        (bind _returnvalue (Animation|PlayAnimMontage "/Game/CityofBrass_Enemies/Meshes/Enemy/Corpse/animation/SkullDeathMontage.SkullDeathMontage" 1.0 "None"))
        (Components|Activation|Activate (Variables|Default|GetNiagara) false)
        (Audio|PlaySoundatLocation "/Game/SoundFX/Skeleton_SFX/Explosion/SkeletonDeath_Cue.SkeletonDeath_Cue" (Transformation|GetActorLocation) "0, 0, 0" 1.0 1.0 0.0 0 0 0 0)
        (Utilities|FlowControl|Delay _returnvalue)
        (for (_array_element _array_index) _enemiesref
          (if (== _array_element self)
            (Utilities|Array|RemoveIndex _enemiesref _array_index)
            (CallFunction|SpawnItem)
            (Game|SpawnActorfromClass "/Game/Blueprints/PS_Explosion.PS_Explosion_C" (Transformation|GetActorTransform) "Undefined" "OverrideRootScale" 0 0)
            (Audio|PlaySoundatLocation "/Game/SoundFX/Skeleton_SFX/Explosion/Explosion_Cue.Explosion_Cue" (Transformation|GetActorLocation) "0, 0, 0" 1.0 1.0 0.0 0 0 0 0)
            (Actor|DestroyActor)))))
    (else
      (bind _returnvalue_2 (Animation|PlayAnimMontage "/Game/CityofBrass_Enemies/Meshes/Enemy/Corpse/animation/Corpse_Flinch.Corpse_Flinch" 1.0 "None"))
      ;;[0.1367 1 0.3032] Show health bar above enemy
      (Rendering|SetVisibility _health true false)
      (Utilities|FlowControl|Delay _returnvalue_2)
      (Rendering|SetVisibility _health false false))))

(fn ConstructionScript)

(fn SpawnItem
  (bind _returnvalue (Transformation|GetActorTransform))
  (bind _returnvalue_2 (Math|Random|RandomInteger 3))
  ;[1 0.1332 0.6061] Conditions to spawn the Health Item
  (if (and (== (Math|Random|RandomInteger 5) 1) (< (Variables|/Game/ThirdPersonBP/Blueprints/Mycharacter.Mycharacter_C|GetHealth (Variables|Default|GetPlayerRef)) 1e+02))
    (Game|SpawnActorfromClass "/Game/ThirdPersonBP/Blueprints/HealItem/BP_HealthItem.BP_HealthItem_C" (Math|Transform|MakeTransform (.location _returnvalue) (.rotation _returnvalue) "0.500000,0.500000,0.500000") "Undefined" "OverrideRootScale" 0 0)
    (elif (or (== _returnvalue_2 2) (== _returnvalue_2 3))
      (Game|SpawnActorfromClass "/Game/ThirdPersonBP/Blueprints/AmmoArrowItem/BP_Arrowammo.BP_Arrowammo_C" (Math|Transform|MakeTransform (.location _returnvalue) (.rotation _returnvalue) "1.000000,1.000000,1.000000") "Undefined" "OverrideRootScale" 0 0))))