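; AI controller for enemy pawns that finds the player, closes in and attacks.
; A looping timer caches the player through a sphere overlap, then moves toward and focuses on them, clearing focus if the move fails.
; Unless flinching, the enemy waits randomly, repositions near the player and calls Attack on BP_EnemyCharacter when close enough.
; The Deambular wander fallback is empty; its random-move logic is disconnected.
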(event Custom|Deambular
  ;[0.4253 1 0.5549] Comment
)

(event Custom|AI%20Process
  (bind _returnvalue (Pawn|GetControlledPawn))
  (Variables|Default|GetPlayer ; Is is an acor with info
    (:then
      (AI|AIMoveTo _returnvalue "0, 0, 0" (Variables|Default|GetPlayer) 3e+02 false :!label _label
        (:OnSuccess
          (AI|SetFocus (Variables|Default|GetPlayer)) ; Set focus on our player
          ;[1 0.38 1 0.62] Verify if is doing flinching animation
          (if (not (Variables|/Game/Blueprints/BP_EnemyCharacter.BP_EnemyCharacter_C|GetIsFlinching (.AsBP%20Enemy%20Character (Utilities|Casting|CastToBP_EnemyCharacter _returnvalue))))
            (|MovingEnemiesandAttack)))
        (:OnFail
          ;[1 1 1 1 12] Do not look at the player
          (AI|ClearFocus) ; When the enemy is not in the Acceptance Radius
        )))
    (:else
      ;[0.3344 0.07011 1] Make a sphere to detect actors
      (bind _outactors (Collision|SphereOverlapActors "0, 0, 0" 1e+04 (Utilities|Array|MakeArray "ObjectTypeQuery3") 0 (Utilities|Array|MakeArray (Pawn|GetControlledPawn))))
      ;[0.8554 0.3475 1] If finds player the searching will be break
      (bind _array_element (Utilities|Array|ForEachLoopwithBreak _outactors :!label _label_2)
        (:LoopBody
          (bind _asmycharacter (Utilities|Casting|CastToMycharacter _array_element))
          (if (Class|Controller|IsPlayerController (Pawn|GetController _asmycharacter))
            (Variables|Default|SetPlayer _asmycharacter)
            (goto _label_2 Break)))
        (:Completed
          (Variables|Default|GetPlayer ; Is is an acor with info
            (:then
              (goto _label))
            (:else
              (CallFunction|Deambular))))))))

(event EventBeginPlay
  (Utilities|Time|SetTimerbyEvent (delegate Custom|AI%20Process) 1.0 true))

(fn ConstructionScript)